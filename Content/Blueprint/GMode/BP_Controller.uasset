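; Player controller that turns input into movement, look, jump and web attach/detach actions on BP_Character, branching on its Walk or Climb status.
; Walking follows the camera's forward and right vectors.
; Climbing sweeps the actor along world up and sideways along the wall from its collision normal, notifying BPRotation, with delta time added to ClimbSpeed rather than multiplied.
; Jumping from a climb launches the character backward at an angle and restores Walk.
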(event `InputAxis|Forward`
  (params (AxisValue :type "Float (single-precision)"))
  (`self.ForwardMoviment` AxisValue))

(event `InputAxis|Right`
  (params (AxisValue :type "Float (single-precision)"))
  (`self.RightMoviment` AxisValue))

(event `InputAction|Jump`
  (params (Key :type "Key Structure"))
  (bind _asbp_character (`/Game/Blueprint/GMode/BP_BasicFunction.GetBasicCharacter`))
  (bind _asbp_character_2 (`/Game/Blueprint/GMode/BP_BasicFunction.GetBasicCharacter`))
  (:`Pressed`
    (switch `/Game/Enum/EN_MovimentStatus` (`/Game/Blueprint/GMode/BP_Character.Moviment Status` _asbp_character)
      (:`NewEnumerator0`
        (`Character.Jump` _asbp_character_2))
      (:`NewEnumerator1`
        (`Character.LaunchCharacter` _asbp_character (`KismetMathLibrary.RotateAngleAxis` (* (`self.GetActorForwardVector` _asbp_character) -800.0) 45.0 (`self.GetActorRightVector` _asbp_character)) false false)
        (`/Game/Blueprint/GMode/BP_Character.SetMovementStatus` _asbp_character_2 "NewEnumerator0")))))

(event `InputAxis|PitchMove`
  (params (AxisValue :type "Float (single-precision)"))
  (`Pawn.AddControllerPitchInput` (`/Game/Blueprint/GMode/BP_BasicFunction.GetBasicCharacter`) AxisValue))

(event `InputAxis|YawMove`
  (params (AxisValue :type "Float (single-precision)"))
  (`Pawn.AddControllerYawInput` (`/Game/Blueprint/GMode/BP_BasicFunction.GetBasicCharacter`) AxisValue))

(event `InputAction|SpiderWeb`
  (params (Key :type "Key Structure"))
  (bind _asbp_character (`/Game/Blueprint/GMode/BP_BasicFunction.GetBasicCharacter`))
  (:`Pressed`
    (`/Game/Blueprint/GMode/BP_Character.AttachWeb` _asbp_character))
  (:`Released`
    (`/Game/Blueprint/GMode/BP_Character.DetachWeb` _asbp_character)))

(fn `ForwardMoviment`
  (params (B :type "Float (double-precision)"))
  (bind _asbp_character (`/Game/Blueprint/GMode/BP_BasicFunction.GetBasicCharacter`))
  (switch `/Game/Enum/EN_MovimentStatus` (`/Game/Blueprint/GMode/BP_Character.Moviment Status` _asbp_character)
    (:`NewEnumerator0`
      (`PawnMovementComponent.AddInputVector` (`Character.CharacterMovement` _asbp_character) (* (`SceneComponent.GetForwardVector` (`/Game/Blueprint/GMode/BP_Character.Camera` _asbp_character)) B) false))
    (:`NewEnumerator1`
      (`self.K2_AddActorWorldOffset` (`/Game/Blueprint/GMode/BP_BasicFunction.GetBasicCharacter`) (* (* (0.0 0.0 1.0) (`local.B`)) (+ (`/Game/Blueprint/GMode/BP_Character.ClimbSpeed` (`/Game/Blueprint/GMode/BP_BasicFunction.GetBasicCharacter`)) (`GameplayStatics.GetWorldDeltaSeconds`))) true false)
      (`/Game/Blueprint/GMode/BP_Rotation.ClimbForward` (`/Game/Blueprint/GMode/BP_Character.BP_Rotation` (`/Game/Blueprint/GMode/BP_BasicFunction.GetBasicCharacter`)) (`local.B`)))))

(fn `RightMoviment`
  (params (B :type "Float (double-precision)"))
  (bind _asbp_character (`/Game/Blueprint/GMode/BP_BasicFunction.GetBasicCharacter`))
  (bind _asbp_character_2 (`/Game/Blueprint/GMode/BP_BasicFunction.GetBasicCharacter`))
  (bind _asbp_character_3 (`/Game/Blueprint/GMode/BP_BasicFunction.GetBasicCharacter`))
  (switch `/Game/Enum/EN_MovimentStatus` (`/Game/Blueprint/GMode/BP_Character.Moviment Status` _asbp_character_2)
    (:`NewEnumerator0`
      (`PawnMovementComponent.AddInputVector` (`Character.CharacterMovement` _asbp_character) (* (`SceneComponent.GetRightVector` (`/Game/Blueprint/GMode/BP_Character.Camera` _asbp_character)) (`local.B`)) false))
    (:`NewEnumerator1`
      (`self.K2_AddActorWorldOffset` _asbp_character_3 (* (* (`KismetMathLibrary.RotateAngleAxis` (`/Game/Blueprint/GMode/BP_Character.CollisionWallNormal` _asbp_character_2) -90.0 (0.0 0.0 1.0)) (`local.B`)) (+ (`/Game/Blueprint/GMode/BP_Character.ClimbSpeed` (`/Game/Blueprint/GMode/BP_BasicFunction.GetBasicCharacter`)) (`GameplayStatics.GetWorldDeltaSeconds`))) true false)
      (`/Game/Blueprint/GMode/BP_Rotation.ClimbRight` (`/Game/Blueprint/GMode/BP_Character.BP_Rotation` _asbp_character_3) (`local.B`)))))

(fn `UserConstructionScript`)