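; Player or NPC character Blueprint that switches between walk, climb and edge movement states for climbing buildings.
; A head-on capsule hit on a BP_Building starts Climb, lifting the character, turning it to face the wall and storing the wall normal.
; SetMovementStatus toggles gravity and a custom collision channel for Walk and Climb, zeroing velocity on climb.
; A capsule overlap during Climb sets Edge, which only has a debug print so far.
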(event `self.ReceiveTick`
  (params (DeltaSeconds :type "Float (single-precision)")))

(event `self.CapsuleComponent.OnComponentHit`
  (params (HitComponent :type "PrimitiveComponent Object Reference") (OtherActor :type "Actor Object Reference") (OtherComp :type "PrimitiveComponent Object Reference") (NormalImpulse :type "Vector Structure") (Hit :type "HitResult Structure (by ref)"))
  (cast `/Game/Blueprint/BP_Building` OtherActor)
  (if (== Hit_Normal (* (`self.GetActorForwardVector`) -1.0) :`ErrorTolerance` 0.2)
    (`self.SetMovementStatus` "NewEnumerator1")
    (set `self.CollisionWallNormal` Hit_Normal)
    (`self.K2_SetActorLocation` (+ (`self.K2_GetActorLocation`) (0.0 0.0 50.0)))
    (`self.K2_SetActorRotation` (`KismetMathLibrary.MakeRotationFromAxes` (* Hit_Normal -1.0)) true)))

(event `self.CapsuleComponent.OnComponentBeginOverlap`
  (params (OverlappedComponent :type "PrimitiveComponent Object Reference") (OtherActor :type "Actor Object Reference") (OtherComp :type "PrimitiveComponent Object Reference") (OtherBodyIndex :type Integer) (bFromSweep :type Boolean) (SweepResult :type "HitResult Structure (by ref)"))
  (switch `/Game/Enum/EN_MovimentStatus` (`self.Moviment Status`)
    (:`NewEnumerator1`
      (`self.SetMovementStatus` "NewEnumerator4")
      (`KismetSystemLibrary.PrintString` "Hello"))))

(fn `SetMovementStatus`
  (params (`Moviment Status` :type "/Game/Enum/EN_MovimentStatus Enum" :default "NewEnumerator0"))
  (bind (_returnvalue_roll _returnvalue_pitch _returnvalue_yaw) (`KismetMathLibrary.BreakRotator` (`self.K2_GetActorRotation`)))
  (if (!= `Moviment Status` (`self.Moviment Status`))
    (bind _output_get (set `self.Moviment Status` `Moviment Status`))
    (switch `/Game/Enum/EN_MovimentStatus` _output_get
      (:`NewEnumerator0`
        (set `CharacterMovementComponent.GravityScale` 1.0 (`self.CharacterMovement`))
        (`PrimitiveComponent.SetCollisionResponseToChannel` (`self.CapsuleComponent`) "ECC_GameTraceChannel1" "ECR_Block")
        (`self.K2_SetActorRotation` (`KismetMathLibrary.MakeRotator` 0.0 _returnvalue_pitch _returnvalue_yaw)))
      (:`NewEnumerator1`
        (set `CharacterMovementComponent.GravityScale` 0.0 (`self.CharacterMovement`))
        (`PrimitiveComponent.SetCollisionResponseToChannel` (`self.CapsuleComponent`) "ECC_GameTraceChannel1" "ECR_Ignore")
        (set `MovementComponent.Velocity` (0.0 0.0 0.0) (`self.CharacterMovement`)))
      (:`NewEnumerator4`))))

(fn `UserConstructionScript`)