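; BP_Rotation smoothly rolls the player character to face the input direction while climbing.
; ClimbForward and ClimbRight input events store the axis values.
; When the character's MovimentStatus is Climb, Tick converts those values to a roll angle with Atan2, holding the current roll without input.
; A fixed-alpha shortest-path lerp applies it each frame, preserving pitch and yaw, so turn speed depends on frame rate.
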(event `self.ReceiveTick`
  (params (DeltaSeconds :type "Float (single-precision)"))
  (bind _asbp_character (`/Game/Blueprint/GMode/BP_BasicFunction.GetBasicCharacter`))
  (bind _climbrightvalue (`self.ClimbRightValue`))
  (bind _climbforwardvalue (`self.ClimbForwardValue`))
  (bind (_returnvalue_roll _returnvalue_pitch _returnvalue_yaw) (`KismetMathLibrary.BreakRotator` (`Actor.K2_GetActorRotation` _asbp_character)))
  (switch `/Game/Enum/EN_MovimentStatus` (`/Game/Blueprint/GMode/BP_Character.Moviment Status` (`/Game/Blueprint/GMode/BP_BasicFunction.GetBasicCharacter`))
    (:`NewEnumerator1`
      (`Actor.K2_SetActorRotation` _asbp_character (`KismetMathLibrary.MakeRotator` (.roll (`KismetMathLibrary.RLerp` (`KismetMathLibrary.MakeRotator` _returnvalue_roll _returnvalue_pitch _returnvalue_yaw) (`KismetMathLibrary.MakeRotator` (select `bool` (and (== _climbrightvalue 0.0) (== _climbforwardvalue 0.0)) :`false` (`KismetMathLibrary.DegAtan2` _climbrightvalue _climbforwardvalue) :`true` _returnvalue_roll) _returnvalue_pitch _returnvalue_yaw) 0.1 true)) (.pitch (`KismetMathLibrary.RLerp` (`KismetMathLibrary.MakeRotator` _returnvalue_roll _returnvalue_pitch _returnvalue_yaw) (`KismetMathLibrary.MakeRotator` (select `bool` (and (== _climbrightvalue 0.0) (== _climbforwardvalue 0.0)) :`false` (`KismetMathLibrary.DegAtan2` _climbrightvalue _climbforwardvalue) :`true` _returnvalue_roll) _returnvalue_pitch _returnvalue_yaw) 0.1 true)) (.yaw (`KismetMathLibrary.RLerp` (`KismetMathLibrary.MakeRotator` _returnvalue_roll _returnvalue_pitch _returnvalue_yaw) (`KismetMathLibrary.MakeRotator` (select `bool` (and (== _climbrightvalue 0.0) (== _climbforwardvalue 0.0)) :`false` (`KismetMathLibrary.DegAtan2` _climbrightvalue _climbforwardvalue) :`true` _returnvalue_roll) _returnvalue_pitch _returnvalue_yaw) 0.1 true))) false))))

(event `ClimbForward`
  (params (ClimbForward :type "Float (double-precision)"))
  (set `self.ClimbForwardValue` ClimbForward))

(event `ClimbRight`
  (params (ClimbRight :type "Float (double-precision)"))
  (set `self.ClimbRightValue` ClimbRight))